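; Projectile actor that explodes on impact or after a three-second fuse, whichever comes first.
; Both the Hit event and the BeginPlay delay feed a shared Explode event at the hit point or the actor's location.
; Explode spawns a particle explosion, applies radial damage with falloff credited to the owner, destroys the actor, and draws debug spheres for the inner and outer damage radii.
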(event `self.ReceiveBeginPlay`
  (`KismetSystemLibrary.Delay` 3.0)
  (`self.Explode` (`self.K2_GetActorLocation`)))

(event `self.ReceiveHit`
  (params (MyComp :type "PrimitiveComponent Object Reference") (Other :type "Actor Object Reference") (OtherComp :type "PrimitiveComponent Object Reference") (bSelfMoved :type Boolean) (HitLocation :type "Vector Structure") (HitNormal :type "Vector Structure") (NormalImpulse :type "Vector Structure") (Hit :type "HitResult Structure (by ref)"))
  (`self.Explode` HitLocation))

(event `Explode`
  (params (Location :type "Vector Structure"))
  (`GameplayStatics.SpawnEmitterAtLocation` "/Game/WeaponEffects/Explosion/P_Explosion.P_Explosion" Location)
  (`GameplayStatics.ApplyRadialDamageWithFalloff` :`BaseDamage` 50.0 :`MinimumDamage` 5.0 :`Origin` Location :`DamageInnerRadius` 60.0 :`DamageOuterRadius` 150.0 :`DamageFalloff` 1.0 :`DamageCauser` (`self.GetOwner`))
  (`|ExecutionSequence`
    (:`then_0`
      (`self.K2_DestroyActor`))
    (:`then_1`
      (`KismetSystemLibrary.DrawDebugSphere` Location 60.0 24 (struct :`R` 1.0 :`A` 1.0) 3.0 1.0)
      (`KismetSystemLibrary.DrawDebugSphere` Location 150.0 24 (struct :`R` 1.0 :`G` 1.0 :`B` 1.0 :`A` 1.0) 3.0 1.0))))

(fn `UserConstructionScript`)